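; Pickable coin Blueprint in the door and key system, offering silver, gold and platinum variants through a CoinType setting.
; The construction script picks CoinMesh from the coin type before running the parent construction script.
; It then sets Value from the matching per-type value variable, so one setting drives both mesh and worth.
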(fn `UserConstructionScript`
  (locals (_SilverValue :type Integer :default 1) (_GoldValue :type Integer :default 10) (_PlatinumValue :type Integer :default 100))
  (bind _cointype (`self.CoinType`))
  (set `self.CoinMesh` (select `/Game/Logic/DoorAndKeySystem/E_CoinType` _cointype :`NewEnumerator0` (`self.Silver`) :`NewEnumerator1` (`self.Gold`) :`NewEnumerator2` (`self.Platimun`)))
  (`parent.UserConstructionScript`)
  (set `self.Value` (select `/Game/Logic/DoorAndKeySystem/E_CoinType` _cointype :`NewEnumerator0` (`local._SilverValue`) :`NewEnumerator1` (`local._GoldValue`) :`NewEnumerator2` (`local._PlatinumValue`))))