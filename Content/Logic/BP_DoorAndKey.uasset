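; BP_DoorAndKey is a door puzzle: the door unlocks after key pickup and at least five coins.
; Key overlap fires once, destroys the key, sets the open flag and fades the door's material opacity.
; Coin overlaps destroy the coin components and update counts in a HUD widget, which also holds the coin total.
; Door overlap turns it green and disables collision when requirements are met, otherwise red.
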(event `self.ReceiveBeginPlay`
  (bind _returnvalue (`|CreateWidget` "/Game/Logic/WBP_DoorHLD.WBP_DoorHLD_C"))
  (set `self.VWidget` _returnvalue)
  (`UserWidget.AddToViewport` _returnvalue 0))

(event `self.KeyCell.OnComponentBeginOverlap`
  (params (OverlappedComponent :type "PrimitiveComponent Object Reference") (OtherActor :type "Actor Object Reference") (OtherComp :type "PrimitiveComponent Object Reference") (OtherBodyIndex :type Integer) (bFromSweep :type Boolean) (SweepResult :type "HitResult Structure (by ref)"))
  (`/Engine/EditorBlueprintResources/StandardMacros.DoOnce` false
    (:`Completed`
      (set `self.Open` true)
      (`ActorComponent.K2_DestroyComponent` (`self.Key`))
      (`MeshComponent.SetScalarParameterValueOnMaterials` (`self.Door`) "Opacity" 0.4)
      (set `/Game/Logic/WBP_DoorHLD.KeyAmount` (+ (`/Game/Logic/WBP_DoorHLD.KeyAmount` (`self.VWidget`)) 1) (`self.VWidget`))
      (`/Game/Logic/WBP_DoorHLD.RefreshKey` (`self.VWidget`)))))

(event `self.DoorCell.OnComponentBeginOverlap`
  (params (OverlappedComponent :type "PrimitiveComponent Object Reference") (OtherActor :type "Actor Object Reference") (OtherComp :type "PrimitiveComponent Object Reference") (OtherBodyIndex :type Integer) (bFromSweep :type Boolean) (SweepResult :type "HitResult Structure (by ref)"))
  (if (and (`self.Open`) (>= (`/Game/Logic/WBP_DoorHLD.CoinAmount` (`self.VWidget`)) 5))
    (`PrimitiveComponent.SetCollisionEnabled` (`self.Door`) "NoCollision")
    (`MeshComponent.SetVectorParameterValueOnMaterials` (`self.Door`) "Color" (0.0 1.0 0.0))
    (else
      (`MeshComponent.SetVectorParameterValueOnMaterials` (`self.Door`) "Color" (1.0 0.0 0.0)))))

(event `self.CoinCall.OnComponentBeginOverlap`
  (params (OverlappedComponent :type "PrimitiveComponent Object Reference") (OtherActor :type "Actor Object Reference") (OtherComp :type "PrimitiveComponent Object Reference") (OtherBodyIndex :type Integer) (bFromSweep :type Boolean) (SweepResult :type "HitResult Structure (by ref)"))
  (set `/Game/Logic/WBP_DoorHLD.CoinAmount` (+ (`/Game/Logic/WBP_DoorHLD.CoinAmount` (`self.VWidget`)) 1) (`self.VWidget`))
  (`ActorComponent.K2_DestroyComponent` OverlappedComponent)
  (`ActorComponent.K2_DestroyComponent` (`SceneComponent.GetAttachParent` OverlappedComponent))
  (`/Game/Logic/WBP_DoorHLD.RefreshCoin` (`self.VWidget`)))

(fn `UserConstructionScript`)