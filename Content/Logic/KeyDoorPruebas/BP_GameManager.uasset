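; BP_GameManager tracks the coin and key totals for a key-and-door test setup.
; At BeginPlay it finds the BP_UIManager with GetActorOfClass and stores it as HUD.
; ProcesaImpactoUniversal switches on the object type (Moneda or Llave), increments the matching counter and calls that counter's refresh on the UI manager's HUD.
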(event `self.ReceiveBeginPlay`
  (bind _returnvalue (`GameplayStatics.GetActorOfClass` "/Game/Logic/BP_UIManager.BP_UIManager_C"))
  (set `self.HUD` _returnvalue))

(fn `ProcesaImpactoUniversal`
  (params (TipoObjeto :type "/Game/Logic/E_TipoObjeto Enum" :default "NewEnumerator0"))
  (bind _returnvalue (+ (select `/Game/Logic/E_TipoObjeto` TipoObjeto :`NewEnumerator0` (`self.TotalCoin`) :`NewEnumerator1` (`self.TotalKey`)) 1))
  (switch `/Game/Logic/E_TipoObjeto` TipoObjeto
    (:`NewEnumerator0`
      (set `self.TotalCoin` _returnvalue)
      (`/Game/Logic/WBP_GamePlayUi.RefreshCoin` (`/Game/Logic/BP_UIManager.HUD` (`self.HUD`))))
    (:`NewEnumerator1`
      (set `self.TotalKey` _returnvalue)
      (`/Game/Logic/WBP_GamePlayUi.RefreshKey` (`/Game/Logic/BP_UIManager.HUD` (`self.HUD`))))))

(fn `UserConstructionScript`)