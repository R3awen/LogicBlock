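; Key-and-door puzzle actor that unlocks passage once the player has the key and at least five coins.
; Key cell overlap fires once, setting Open, destroying the key, lowering door opacity and updating the key count on the HUD from BP_UIManager.
; Door cell overlap checks Open and HUD coins, then disables collision and turns the door green, or otherwise red.
; Coin pickup logic remains disconnected.
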(event `self.ReceiveBeginPlay`
  ; Ui
  (bind _returnvalue (`GameplayStatics.GetActorOfClass` "/Game/Logic/BP_UIManager.BP_UIManager_C"))
  (set `self.HUD` (`/Game/Logic/BP_UIManager.HUD` _returnvalue)))

(event `self.KeyCell.OnComponentBeginOverlap`
  (params (OverlappedComponent :type "PrimitiveComponent Object Reference") (OtherActor :type "Actor Object Reference") (OtherComp :type "PrimitiveComponent Object Reference") (OtherBodyIndex :type Integer) (bFromSweep :type Boolean) (SweepResult :type "HitResult Structure (by ref)"))
  ; Key
  (`/Engine/EditorBlueprintResources/StandardMacros.DoOnce` false
    (:`Completed`
      (set `self.Open` true)
      (`ActorComponent.K2_DestroyComponent` (`self.Key`))
      (`MeshComponent.SetScalarParameterValueOnMaterials` (`self.Door`) "Opacity" 0.4)
      (set `/Game/Logic/WBP_GamePlayUi.KeyAmount` (+ (`/Game/Logic/WBP_GamePlayUi.KeyAmount` (`self.HUD`)) 1) (`self.HUD`))
      (`/Game/Logic/WBP_GamePlayUi.RefreshKey` (`self.HUD`)))))

(event `self.DoorCell.OnComponentBeginOverlap`
  (params (OverlappedComponent :type "PrimitiveComponent Object Reference") (OtherActor :type "Actor Object Reference") (OtherComp :type "PrimitiveComponent Object Reference") (OtherBodyIndex :type Integer) (bFromSweep :type Boolean) (SweepResult :type "HitResult Structure (by ref)"))
  ; Door
  (if (and (`self.Open`) (>= (`/Game/Logic/WBP_GamePlayUi.CoinAmount` (`self.HUD`)) 5))
    (`PrimitiveComponent.SetCollisionEnabled` (`self.Door`) "NoCollision")
    (`MeshComponent.SetVectorParameterValueOnMaterials` (`self.Door`) "Color" (0.0 1.0 0.0))
    (else
      (`MeshComponent.SetVectorParameterValueOnMaterials` (`self.Door`) "Color" (1.0 0.0 0.0)))))

(event `self.CoinCall.OnComponentBeginOverlap`
  (params (OverlappedComponent :type "PrimitiveComponent Object Reference") (OtherActor :type "Actor Object Reference") (OtherComp :type "PrimitiveComponent Object Reference") (OtherBodyIndex :type Integer) (bFromSweep :type Boolean) (SweepResult :type "HitResult Structure (by ref)"))
  ; Coin No necesario
)

(fn `UserConstructionScript`)