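; BP_Camera is a standalone camera actor that follows the third-person player character.
; On BeginPlay it sets itself as the player controller's view target and caches the BP_ThirdPersonCharacter it finds.
; Each Tick it uses VInterpTo to glide toward the character's position plus a camera offset and a look-ahead along its forward vector, without changing rotation.
; An alternative axis-by-axis follow approach remains in the graph but never runs.
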(event `self.ReceiveBeginPlay`
  ; Iniciazar la camara
  (`PlayerController.SetViewTargetWithBlend` (`GameplayStatics.GetPlayerController` 0) self 0.0 "VTBlend_Linear" 0.0 false)
  (bind _returnvalue (`GameplayStatics.GetActorOfClass` "/Game/ThirdPerson/Blueprints/BP_ThirdPersonCharacter.BP_ThirdPersonCharacter_C"))
  (set `self.CharTarget` _returnvalue))

(event `self.ReceiveTick`
  (params (DeltaSeconds :type "Float (single-precision)"))
  (bind _chartarget (`self.CharTarget`))
  ; Seguir al personaje con la camara
  (`self.K2_SetActorLocation` (`KismetMathLibrary.VInterpTo` (`self.K2_GetActorLocation`) (+ (`SceneComponent.K2_GetComponentLocation` (`Actor.RootComponent` _chartarget)) (`self.CameraOffset`) (* (`self.GetActorForwardVector` _chartarget) (`self.LookAheadDistance`)) (0.0 0.0 0.0)) DeltaSeconds (`self.FollowSpeed`))))

(fn `UserConstructionScript`)